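; Player controller for a Snake game that turns keyboard or gamepad input into direction changes for two players.
; On BeginPlay it registers an Enhanced Input mapping context on the local player subsystem.
; Separate move actions for each player call SetDirection or SetDirectionPlayer2 with up, down, left or right, so one controller drives both players locally.
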(event Input|EnhancedActionEvents|EnhancedInputActionIA_MoveDown
  (params (ActionValue :type Boolean) (ElapsedSeconds :type Float%20%28double-precision%29) (TriggeredSeconds :type Float%20%28double-precision%29) (InputAction :type Input%20Action%20Object%20Reference :default "/Game/Blueprints/Inputs/Actions/IA_MoveDown.IA_MoveDown"))
  (Class|SnakePlayerController|SetDirection "Down"))

(event Input|EnhancedActionEvents|EnhancedInputActionIA_MoveDownPlayer2
  (params (ActionValue :type Boolean) (ElapsedSeconds :type Float%20%28double-precision%29) (TriggeredSeconds :type Float%20%28double-precision%29) (InputAction :type Input%20Action%20Object%20Reference :default "/Game/Blueprints/Inputs/Actions/IA_MoveDownPlayer2.IA_MoveDownPlayer2"))
  (Class|SnakePlayerController|SetDirectionPlayer2 "Down"))

(event Input|EnhancedActionEvents|EnhancedInputActionIA_MoveLeft
  (params (ActionValue :type Boolean) (ElapsedSeconds :type Float%20%28double-precision%29) (TriggeredSeconds :type Float%20%28double-precision%29) (InputAction :type Input%20Action%20Object%20Reference :default "/Game/Blueprints/Inputs/Actions/IA_MoveLeft.IA_MoveLeft"))
  (Class|SnakePlayerController|SetDirection "Left"))

(event Input|EnhancedActionEvents|EnhancedInputActionIA_MoveLeftPlayer2
  (params (ActionValue :type Boolean) (ElapsedSeconds :type Float%20%28double-precision%29) (TriggeredSeconds :type Float%20%28double-precision%29) (InputAction :type Input%20Action%20Object%20Reference :default "/Game/Blueprints/Inputs/Actions/IA_MoveLeftPlayer2.IA_MoveLeftPlayer2"))
  (Class|SnakePlayerController|SetDirectionPlayer2 "Left"))

(event Input|EnhancedActionEvents|EnhancedInputActionIA_MoveRight
  (params (ActionValue :type Boolean) (ElapsedSeconds :type Float%20%28double-precision%29) (TriggeredSeconds :type Float%20%28double-precision%29) (InputAction :type Input%20Action%20Object%20Reference :default "/Game/Blueprints/Inputs/Actions/IA_MoveRight.IA_MoveRight"))
  (Class|SnakePlayerController|SetDirection "Right"))

(event Input|EnhancedActionEvents|EnhancedInputActionIA_MoveRightPlayer2
  (params (ActionValue :type Boolean) (ElapsedSeconds :type Float%20%28double-precision%29) (TriggeredSeconds :type Float%20%28double-precision%29) (InputAction :type Input%20Action%20Object%20Reference :default "/Game/Blueprints/Inputs/Actions/IA_MoveRightPlayer2.IA_MoveRightPlayer2"))
  (Class|SnakePlayerController|SetDirectionPlayer2 "Right"))

(event Input|EnhancedActionEvents|EnhancedInputActionIA_MoveUp
  (params (ActionValue :type Boolean) (ElapsedSeconds :type Float%20%28double-precision%29) (TriggeredSeconds :type Float%20%28double-precision%29) (InputAction :type Input%20Action%20Object%20Reference :default "/Game/Blueprints/Inputs/Actions/IA_MoveUp.IA_MoveUp"))
  (Class|SnakePlayerController|SetDirection "Up"))

(event Input|EnhancedActionEvents|EnhancedInputActionIA_MoveUpPlayer2
  (params (ActionValue :type Boolean) (ElapsedSeconds :type Float%20%28double-precision%29) (TriggeredSeconds :type Float%20%28double-precision%29) (InputAction :type Input%20Action%20Object%20Reference :default "/Game/Blueprints/Inputs/Actions/IA_MoveUpPlayer2.IA_MoveUpPlayer2"))
  (Class|SnakePlayerController|SetDirectionPlayer2 "Up"))

(event EventBeginPlay
  (Input|AddMappingContext (PlayerController|LocalPlayerSubsystems|GetEnhancedInputLocalPlayerSubsystem self) "/Game/Blueprints/Inputs/InputMappingContext.InputMappingContext" 0 "(bIgnoreAllPressedKeysUntilRelease=True,bForceImmediately=False,bNotifyUserSettings=False)"))

(event EventTick
  (params (DeltaSeconds :type Float%20%28single-precision%29)))

(fn ConstructionScript)