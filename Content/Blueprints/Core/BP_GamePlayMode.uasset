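; Gameplay game mode for the snake game that spawns and wires up the snake pawns on BeginPlay.
; Player controller 0 possesses the first pawn and receives references to it and the snake world.
; The GameStateSubsystem mode adds a second pawn: AI-controlled through controller 0 in PvE, or possessed by a freshly created local player in PvP.
; Both two-snake modes enable wall hits on each pawn.
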(event EventBeginPlay
  (bind _defaultspawntransformpawn2 (Variables|Default|GetDefaultSpawnTransformPawn2))
  (bind _assnake_player_controller (Utilities|Casting|CastToSnakePlayerController (Game|GetPlayerController 0)))
  (bind _returnvalue (Game|SpawnActorfromClass "/Game/Blueprints/BP_PlayerPawn.BP_PlayerPawn_C" (Variables|Default|GetDefaultSpawnTransform) "Undefined" "MultiplyWithRoot" 0 0))
  (Pawn|Possess _assnake_player_controller _returnvalue)
  (Variables|/Script/MazeProject.SnakePlayerController|Setm_snakePawn1 _assnake_player_controller _returnvalue)
  (bind _returnvalue_2 (Actor|GetActorOfClass "/Game/Blueprints/BP_SnakeWorld.BP_SnakeWorld_C"))
  (Variables|/Script/MazeProject.SnakePlayerController|SetsnakeWorld _assnake_player_controller _returnvalue_2)
  (bind _returnvalue_3 (Class|GameStateSubsystem|GetGameplayMode (Subsystems|GetGameStateSubsystem)))
  (switch Utilities|FlowControl|Switch|SwitchonSnakePlayMode _returnvalue_3
    (:PvE
      (bind _returnvalue_4 (Game|SpawnActorfromClass "/Game/Blueprints/BP_PlayerPawn.BP_PlayerPawn_C" _defaultspawntransformpawn2 "Undefined" "MultiplyWithRoot" 0 0))
      (bind _assnake_player_controller_2 (Utilities|Casting|CastToSnakePlayerController (Game|GetPlayerController 0)))
      (Variables|/Script/MazeProject.SnakePlayerController|Setm_snakePawn2 _assnake_player_controller_2 _returnvalue_4)
      (Variables|/Script/MazeProject.SnakePlayerController|SetisAIControlled _assnake_player_controller_2 true)
      (Class|SnakePlayerController|SetPlayer2AIControlled _assnake_player_controller_2 true)
      ;[0.15 0.15 0.15 0.5] player 2
      (Class|SnakePawn|EnableWallHit _returnvalue_4)
      ;[0.15 0.15 0.15 0.5] player 1
      (Class|SnakePawn|EnableWallHit _returnvalue))
    (:PvP
      (if (Class|KismetSystemLibrary|HasMultipleLocalPlayers)
        (Class|GameplayStatics|RemovePlayer (Game|GetPlayerController 1) true))
      (bind _returnvalue_5 (Class|GameplayStatics|CreatePlayer -1))
      (bind _returnvalue_6 (Game|SpawnActorfromClass "/Game/Blueprints/BP_PlayerPawn.BP_PlayerPawn_C" _defaultspawntransformpawn2 "Undefined" "MultiplyWithRoot" 0 0))
      (Pawn|Possess _returnvalue_5 _returnvalue_6)
      (Variables|/Script/MazeProject.SnakePlayerController|Setm_snakePawn2 _assnake_player_controller _returnvalue_6)
      (Variables|/Script/MazeProject.SnakePlayerController|SetisAIControlled _assnake_player_controller false)
      ;[0.15 0.15 0.15 0.5] player 2
      (Class|SnakePawn|EnableWallHit _returnvalue_6)
      ;[0.15 0.15 0.15 0.5] player 1
      (Class|SnakePawn|EnableWallHit _returnvalue))))

(event EventTick
  (params (DeltaSeconds :type Float%20%28single-precision%29)))

(fn ConstructionScript)